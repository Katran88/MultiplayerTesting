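; BP_BadMedkit is a pickup that changes the player's health on touch, apparently a harmful variant of a medkit.
; When its Collision component begins overlapping a ThirdPersonCharacter, it adds its Hill value to that character's CurrentHelth.
; It clamps the result at zero with no upper limit, which suggests Hill is meant to be negative, then destroys itself.
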(event OnComponentBeginOverlap(Collision)
  (params (OverlappedComponent :type Primitive%20Component%20Object%20Reference) (OtherActor :type Actor%20Object%20Reference) (OtherComp :type Primitive%20Component%20Object%20Reference) (OtherBodyIndex :type Integer) (bFromSweep :type Boolean) (SweepResult :type Hit%20Result%20Structure%20%28by%20ref%29))
  (bind _asthird_person_character (Utilities|Casting|CastToThirdPersonCharacter OtherActor))
  (bind _output_get (Variables|/Game/Blueprints_and_materials/ThirdPersonCharacter.ThirdPersonCharacter_C|SetCurrentHelth _asthird_person_character (+ (Variables|/Game/Blueprints_and_materials/ThirdPersonCharacter.ThirdPersonCharacter_C|GetCurrentHelth _asthird_person_character) (Variables|Default|GetHill))))
  (if (< _output_get 0.0)
    (Variables|/Game/Blueprints_and_materials/ThirdPersonCharacter.ThirdPersonCharacter_C|SetCurrentHelth _asthird_person_character 0.0))
  (Actor|DestroyActor))

(fn ConstructionScript
  (|CallParentFunction))