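; BP_finish is a healing zone that restores a ThirdPersonCharacter's health when it overlaps the Box.
; A delay loop adds 10 health each second until it reaches 100, turning the PointLight green while healing and red when full.
; Leaving the box turns the light red and clears PersonInside, but the live loop never checks that flag, so healing continues.
; An unconnected older loop that checks PersonInside remains unused.
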(event OnComponentBeginOverlap(Box)
  (params (OverlappedComponent :type Primitive%20Component%20Object%20Reference) (OtherActor :type Actor%20Object%20Reference) (OtherComp :type Primitive%20Component%20Object%20Reference) (OtherBodyIndex :type Integer) (bFromSweep :type Boolean) (SweepResult :type Hit%20Result%20Structure%20%28by%20ref%29))
  (bind _asthird_person_character (Utilities|Casting|CastToThirdPersonCharacter OtherActor))
  (if (< (Variables|/Game/Blueprints_and_materials/ThirdPersonCharacter.ThirdPersonCharacter_C|GetCurrentHelth _asthird_person_character) 1e+02) :!label _label
    (Utilities|FlowControl|Delay 1.0)
    (Rendering|Components|Light|SetLightColor (Variables|Default|GetPointLight) "(R=0.106083,G=0.695833,B=0.063703,A=1.000000)" true)
    (bind _output_get (Variables|/Game/Blueprints_and_materials/ThirdPersonCharacter.ThirdPersonCharacter_C|SetCurrentHelth _asthird_person_character (+ (Variables|/Game/Blueprints_and_materials/ThirdPersonCharacter.ThirdPersonCharacter_C|GetCurrentHelth _asthird_person_character) 1e+01)))
    (if (< _output_get 1e+02)
      (goto _label)
      (else
        (Rendering|Components|Light|SetLightColor (Variables|Default|GetPointLight) "(R=1.000000,G=0.015209,B=0.000000,A=1.000000)" true)))
    (else
      (Variables|Default|Setperson%20inside false))))

(event OnComponentEndOverlap(Box)
  (params (OverlappedComponent :type Primitive%20Component%20Object%20Reference) (OtherActor :type Actor%20Object%20Reference) (OtherComp :type Primitive%20Component%20Object%20Reference) (OtherBodyIndex :type Integer))
  (Rendering|Components|Light|SetLightColor (Variables|Default|GetPointLight) "(R=1.000000,G=0.015209,B=0.000000,A=1.000000)" true)
  (Variables|Default|Setperson%20inside false))

(fn ConstructionScript)