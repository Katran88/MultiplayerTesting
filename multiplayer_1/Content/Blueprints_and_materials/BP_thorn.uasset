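; BP_thorn is a thorn hazard that deals periodic damage to a ThirdPersonCharacter inside its Pain_collision volume.
; Beginning overlap subtracts a fixed amount from CurrentHelth and briefly switches on the character's damage effect, then loops through delays while the ActorInside flag stays set.
; Ending overlap clears the flag and switches the damage effect off.
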(event OnComponentBeginOverlap(pain_collision)
  (params (OverlappedComponent :type Primitive%20Component%20Object%20Reference) (OtherActor :type Actor%20Object%20Reference) (OtherComp :type Primitive%20Component%20Object%20Reference) (OtherBodyIndex :type Integer) (bFromSweep :type Boolean) (SweepResult :type Hit%20Result%20Structure%20%28by%20ref%29))
  (bind _asthird_person_character (Utilities|Casting|CastToThirdPersonCharacter OtherActor :!label _label))
  (Variables|Default|Setactor _asthird_person_character)
  (Variables|Default|Setactor_inside true)
  (Variables|/Game/Blueprints_and_materials/ThirdPersonCharacter.ThirdPersonCharacter_C|SetCurrentHelth (Variables|Default|Getactor) (- (Variables|/Game/Blueprints_and_materials/ThirdPersonCharacter.ThirdPersonCharacter_C|GetCurrentHelth (Variables|Default|Getactor)) 5.0))
  (Default|DamageEffecton (Variables|Default|Getactor))
  (Utilities|FlowControl|Delay 1.0)
  (Default|DamageEffectOff (Variables|Default|Getactor))
  (if (Variables|Default|Getactor_inside)
    (Utilities|FlowControl|Delay 1.0)
    (if (Variables|Default|Getactor_inside)
      (goto _label))))

(event OnComponentEndOverlap(pain_collision)
  (params (OverlappedComponent :type Primitive%20Component%20Object%20Reference) (OtherActor :type Actor%20Object%20Reference) (OtherComp :type Primitive%20Component%20Object%20Reference) (OtherBodyIndex :type Integer))
  (bind _asthird_person_character (Utilities|Casting|CastToThirdPersonCharacter OtherActor))
  (Variables|Default|Setactor_inside false)
  (Default|DamageEffectOff _asthird_person_character))

(fn ConstructionScript)